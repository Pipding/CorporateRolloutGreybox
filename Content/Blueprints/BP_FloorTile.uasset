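; BP_FloorTile is a floor segment for an endless track that extends as the player moves along it.
; Construction randomly leaves the tile empty or adds a hurdle or limbo child actor at the Arrow's transform.
; When the player character overlaps EndTrigger, the game mode adds another tile, and this one destroys itself after a delay.
; GetAttachPointTransform exposes the AttachPoint's world transform.
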(event `self.EndTrigger.OnComponentBeginOverlap`
  (params (OverlappedComponent :type "PrimitiveComponent Object Reference") (OtherActor :type "Actor Object Reference") (OtherComp :type "PrimitiveComponent Object Reference") (OtherBodyIndex :type Integer) (bFromSweep :type Boolean) (SweepResult :type "HitResult Structure (by ref)"))
  (cast `/Game/ThirdPerson/Blueprints/BP_ThirdPersonCharacter` OtherActor)
  (bind _asbp_third_person_game_mode (cast `/Game/ThirdPerson/Blueprints/BP_ThirdPersonGameMode` (`GameplayStatics.GetGameMode`)))
  (`/Game/ThirdPerson/Blueprints/BP_ThirdPersonGameMode.AddFloorTile` _asbp_third_person_game_mode)
  (`KismetSystemLibrary.Delay` 8.0)
  (`self.K2_DestroyActor`))

(fn `GetAttachPointTransform`
  (returns (ReturnValue :type "Transform Structure"))
  (return (`SceneComponent.K2_GetComponentToWorld` (`self.AttachPoint`))))

(fn `SpawnHurdle`
  (`AddComponent|NODE_AddChildActorComponent-0` :`RelativeTransform` (`SceneComponent.GetRelativeTransform` (`self.Arrow`))))

(fn `SpawnLimbo`
  (`AddComponent|NODE_AddChildActorComponent-1` :`RelativeTransform` (`SceneComponent.GetRelativeTransform` (`self.Arrow`))))

(fn `UserConstructionScript`
  (if (`KismetMathLibrary.RandomBoolWithWeight` 0.6)
    (if (`KismetMathLibrary.RandomBool`)
      (`self.SpawnHurdle`)
      (else
        (`self.SpawnLimbo`)))))