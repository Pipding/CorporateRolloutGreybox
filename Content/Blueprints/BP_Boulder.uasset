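; BP_Boulder is a rolling boulder hazard that chases the player along world +X and kills them on contact.
; Each tick it advances by Speed, unscaled by delta time, and spins its Sphere at a time-scaled rate.
; When the distance reaches MaxDistanceFromPlayer, it first snaps to that far behind the player on X, matching their Y.
; Sphere hits and Box overlaps call Death on BP_ThirdPersonCharacter.
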(event `self.ReceiveTick`
  (params (DeltaSeconds :type "Float (single-precision)"))
  (`self.PursuePlayer` DeltaSeconds))

(event `self.Sphere.OnComponentHit`
  (params (HitComponent :type "PrimitiveComponent Object Reference") (OtherActor :type "Actor Object Reference") (OtherComp :type "PrimitiveComponent Object Reference") (NormalImpulse :type "Vector Structure") (Hit :type "HitResult Structure (by ref)"))
  (bind _asbp_third_person_character (cast `/Game/ThirdPerson/Blueprints/BP_ThirdPersonCharacter` OtherActor))
  (`/Game/ThirdPerson/Blueprints/BP_ThirdPersonCharacter.Death` _asbp_third_person_character))

(event `self.Box.OnComponentBeginOverlap`
  (params (OverlappedComponent :type "PrimitiveComponent Object Reference") (OtherActor :type "Actor Object Reference") (OtherComp :type "PrimitiveComponent Object Reference") (OtherBodyIndex :type Integer) (bFromSweep :type Boolean) (SweepResult :type "HitResult Structure (by ref)"))
  (bind _asbp_third_person_character (cast `/Game/ThirdPerson/Blueprints/BP_ThirdPersonCharacter` OtherActor))
  (`/Game/ThirdPerson/Blueprints/BP_ThirdPersonCharacter.Death` _asbp_third_person_character))

(fn `CatchUpToMaxPlayerDistance`
  (bind (_returnvalue_x _returnvalue_y) (`KismetMathLibrary.BreakVector` (`self.GetPlayerLocation`)))
  (`SceneComponent.K2_SetWorldLocation` (`self.DefaultSceneRoot`) (`KismetMathLibrary.MakeVector` (- _returnvalue_x (`self.MaxDistanceFromPlayer`)) _returnvalue_y) false false))

(fn `MoveBoulderForward`
  (params (DeltaTime :type "Float (double-precision)"))
  (bind (_returnvalue_x _returnvalue_y _returnvalue_z) (`KismetMathLibrary.BreakVector` (`SceneComponent.K2_GetComponentLocation` (`self.DefaultSceneRoot`))))
  (`SceneComponent.K2_SetWorldLocation` (`self.DefaultSceneRoot`) (`KismetMathLibrary.MakeVector` (+ (`self.Speed`) _returnvalue_x) _returnvalue_y _returnvalue_z) false false)
  (`SceneComponent.K2_AddWorldRotation` (`self.Sphere`) (`KismetMathLibrary.MakeRotator` 0.0 (* (`local.DeltaTime`) -180.0)) false false))

(fn `PursuePlayer`
  (params (DeltaTime :type "Float (double-precision)"))
  (if (>= (`self.DistanceToPlayer`) (`self.MaxDistanceFromPlayer`))
    (`self.CatchUpToMaxPlayerDistance`))
  (`self.MoveBoulderForward` DeltaTime))

(fn `UserConstructionScript`)